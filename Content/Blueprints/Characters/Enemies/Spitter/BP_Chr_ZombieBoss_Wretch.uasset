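; Blueprint for the Wretch zombie boss character, an enemy in the Spitter folder that reacts to spotting the player.
; When PawnSensing sees a military-base character, it stores it as Target and snaps its rotation to face it.
; It then writes the SeenPlayer flag and PlayerTarget object to its AI controller's blackboard, presumably for a behavior tree to act on.
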(event `self.PawnSensing.OnSeePawn`
  (params (Pawn :type "Pawn Object Reference"))
  (bind _returnvalue (`AIBlueprintHelperLibrary.GetBlackboard` (`AIBlueprintHelperLibrary.GetAIController` self)))
  (bind _asbp_chr_military_base (cast `/Game/Blueprints/Characters/Players/BP_Chr_MilitaryBase` Pawn))
  (bind _output_get (set `self.Target` _asbp_chr_military_base))
  (`self.K2_SetActorRotation` (`KismetMathLibrary.FindRelativeLookAtRotation` (`KismetMathLibrary.Conv_VectorToTransform` (`self.K2_GetActorLocation`)) (`self.K2_GetActorLocation` _output_get)))
  (`BlackboardComponent.SetValueAsBool` _returnvalue "SeenPlayer" true)
  (`BlackboardComponent.SetValueAsObject` _returnvalue "PlayerTarget" _output_get))

(fn `UserConstructionScript`)