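; Base Blueprint for a boss zombie enemy in the Horder enemy set.
; Tick watches HP and, at zero or below, marks the zombie as not in use and refills HP to 100, recycling it rather than destroying it.
; When PawnSensing sees a military character, it sets SeenPlayer and stores that pawn as PlayerTarget on the AI controller's blackboard.
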(event `self.ReceiveBeginPlay`)

(event `self.ReceiveTick`
  (params (DeltaSeconds :type "Float (single-precision)"))
  (if (<= (`self.HP`) 0.0)
    (`self.SetInUse` false)
    (set `self.HP` 100.0)))

(event `self.PawnSensing.OnSeePawn`
  (params (Pawn :type "Pawn Object Reference"))
  (bind _returnvalue (`AIBlueprintHelperLibrary.GetBlackboard` (`AIBlueprintHelperLibrary.GetAIController` self)))
  ;[1 1 1] Logic on seeing the player
  (bind _asbp_chr_military_base (cast `/Game/Blueprints/Characters/Players/BP_Chr_MilitaryBase` Pawn))
  (`BlackboardComponent.SetValueAsBool` _returnvalue "SeenPlayer" true)
  (`BlackboardComponent.SetValueAsObject` _returnvalue "PlayerTarget" _asbp_chr_military_base))

(fn `UserConstructionScript`)