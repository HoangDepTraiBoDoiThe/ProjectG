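; Actor component that provides an object pool of enemies for spawning without creating new actors at runtime.
; On BeginPlay it pre-spawns actors of the pooled enemy class up to the pool size and marks them unused.
; SpawnFromPool takes the first free enemy via a linear search, moves it to the given transform and marks it in use.
; When none is free, it only prints an error instead of growing the pool.
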(event `self.ReceiveBeginPlay`
  (`self.InitializePool`))

(event `InitializePool`
  (for _ (range (+ (`self.PoolSize`) 1))
    (bind _returnvalue (`|SpawnActorFromClass` (`self.PooledEnemyClass`) (`KismetMathLibrary.MakeTransform` (0.0 0.0 0.0)) "Undefined" "MultiplyWithRoot" null null))
    (`KismetArrayLibrary.Array_AddUnique` (`self.EnemyPool`) _returnvalue)
    (`/Game/Blueprints/Characters/Enemies/PoolingSystem/BP_PooledEnemies.SetInUse` _returnvalue false)))

(fn `FindFirstAvailableEnemy`
  (returns (`Pooled Enemy` :type "/Game/Blueprints/Characters/Enemies/PoolingSystem/BP_PooledEnemies Object Reference"))
  ;[1 1 1] Loop through EnemyPool array, find the first one that is not in use and return it
  (for _array_element (`self.EnemyPool`)
    (if (not (`/Game/Blueprints/Characters/Enemies/PoolingSystem/BP_PooledEnemies.IsInUse` _array_element))
      (return _array_element))))

(fn `SpawnFromPool`
  (params (SpawnTransform :type "Transform Structure"))
  (returns (`Pooled Enemy` :type "/Game/Blueprints/Characters/Enemies/PoolingSystem/BP_PooledEnemies Object Reference"))
  ;[1 1 1] Get the available actors, if it is valid then spawn it and set IsInUse as true
  (bind _pooled_enemy (`self.FindFirstAvailableEnemy`))
  (`/Engine/EditorBlueprintResources/StandardMacros.IsValid` _pooled_enemy
    (:`Is Valid`
      (`Actor.K2_SetActorTransform` _pooled_enemy SpawnTransform false false)
      (`/Game/Blueprints/Characters/Enemies/PoolingSystem/BP_PooledEnemies.SetInUse` _pooled_enemy true)
      (return _pooled_enemy))
    (:`Is Not Valid`
      (`KismetSystemLibrary.PrintString` "Enemy not valid"))))