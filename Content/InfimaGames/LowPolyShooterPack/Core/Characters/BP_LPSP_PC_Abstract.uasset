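; Abstract player controller for Low Poly Shooter Pack that handles the player spawn flow.
; On non-dedicated-server BeginPlay, it either shows the spawn loadout menu to the local controller or covers the screen via the HUD and requests a respawn.
; Spawning destroys any controlled pawn and restarts through the GameMode, while custom spawns forward loadout, attachment and inventory data to it by server event.
; Key-press and gamepad queries are stubs.
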(event `Event Show Spawn Menu`
  ;[1 0.07939 0 1 12] Show Spawn Menu
  (bind _returnvalue (`|CreateWidget` (`self.Spawn Menu Class`) self))
  (`UserWidget.AddToViewport` _returnvalue 0))

(event `Event (Server) Spawn Player Custom`
  (params (`Override Attachments` :type Boolean) (Loadout :type "/Game/InfimaGames/LowPolyShooterPack/Core/Gamemodes/S_LPSP_Loadout Structure") (`Inventory Data` :type "DataTable Object Reference"))
  ;[1 0.9481 0 1 12] Spawn Player
  (message `/Game/InfimaGames/LowPolyShooterPack/Core/Gamemodes/BPI_LPSP_GM.LPSP - Spawn Player Custom` (`GameplayStatics.GetGameMode`) self `Inventory Data` `Override Attachments` Loadout))

(event `Event Server Spawn`
  ;[1 0.4061 0 1 12] Spawn
  (`|ExecutionSequence`
    (:`then_0`
      (`/Engine/EditorBlueprintResources/StandardMacros.IsValid` (`self.K2_GetPawn`)
        (:`Is Valid`
          (`self.K2_DestroyActor` (`self.K2_GetPawn`)))))
    (:`then_1`
      (`GameModeBase.RestartPlayer` (`GameplayStatics.GetGameMode`) self))))

(event `self.ReceiveBeginPlay`
  ;[0.9123 1 0 1 12] Begin Play
  (if (not (`KismetSystemLibrary.IsDedicatedServer`))
    (`self.LPSP - Try Show Spawn Menu`)))

(event `/Game/InfimaGames/LowPolyShooterPack/Core/Characters/BPI_LPSP_Controller.LPSP - Try Show Spawn Menu`
  ;[1 0.8267 0 1 12] Try Show Spawn Menu
  (if (`self.Spawn Loadout Menu`)
    (if (`self.IsLocalPlayerController`)
      (`self.Event Show Spawn Menu`))
    (else
      (message `/Game/InfimaGames/LowPolyShooterPack/Core/Characters/BPI_LPSP_HUD.LPSP - Show Screen Cover` (`self.GetHUD`))
      (`self.Event Server Spawn`))))

(fn `LPSP - Get Key Pressed`
  (returns (Value :type "Key Structure"))
  (return))

(fn `LPSP - Is Using Gamepad`
  (returns (Value :type Boolean))
  (return false))

(fn `UserConstructionScript`)